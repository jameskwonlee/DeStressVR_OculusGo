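; VR guided breathing exercise, started when the player pawn overlaps the BreathRing, which then becomes visible and stops colliding.
; An intro sound plays while the RegularBreaths timeline scales the ring between two sizes.
; A Delay on that timeline's Update leads to a coherent-breathing voiceover and the CoherenceTimer timeline, which takes over scaling.
; Further Delays on its Update hide the ring and open the menu level.
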(event `self.BreathRing.OnComponentBeginOverlap`
  (params (OverlappedComponent :type "PrimitiveComponent Object Reference") (OtherActor :type "Actor Object Reference") (OtherComp :type "PrimitiveComponent Object Reference") (OtherBodyIndex :type Integer) (bFromSweep :type Boolean) (SweepResult :type "HitResult Structure (by ref)"))
  (`self.SetActorTickEnabled` true)
  (if (== (`GameplayStatics.GetObjectClass` OtherActor) "/Game/player/BP_MyVRPawn.BP_MyVRPawn_C")
    (`SceneComponent.SetVisibility` (`self.BreathRing`) true false)
    (`PrimitiveComponent.SetCollisionEnabled` (`self.BreathRing`) "NoCollision")
    (`GameplayStatics.PlaySoundAtLocation` "/Game/audio/VO/BreatheInBreatheOutSimple_Cue.BreatheInBreatheOutSimple_Cue" (`SceneComponent.K2_GetComponentLocation` (`self.SoundSphere`)) (struct) 1.0 1.0 0.0 null null null)
    (bind (_direction _regularbreaths) (`Timeline|Regular Breaths`)
      (:`Update`
        (`SceneComponent.SetRelativeScale3D` (`self.BreathRing`) (`KismetMathLibrary.VLerp` (`self.startingScale`) (`self.endingScale`) _regularbreaths))
        (`KismetSystemLibrary.Delay` 30.0)
        (`GameplayStatics.PlaySoundAtLocation` "/Game/audio/VO/CoherentBreathingVO_Cue.CoherentBreathingVO_Cue" (`SceneComponent.K2_GetComponentLocation` (`self.SoundSphere`)) (struct) 1.0 1.0 0.0 null null null)
        (bind (_direction_2 _alpha) (`Timeline|Coherence Timer`)
          (:`Update`
            (`SceneComponent.SetRelativeScale3D` (`self.BreathRing`) (`KismetMathLibrary.VLerp` (`self.startingScale`) (`self.endingScale`) _alpha))
            (`KismetSystemLibrary.Delay` 120.0)
            (`SceneComponent.SetVisibility` (`self.BreathRing`) false false)
            (`KismetSystemLibrary.Delay` 3.0)
            (`GameplayStatics.OpenLevel` "Level_Menu")))))))

(fn `UserConstructionScript`)